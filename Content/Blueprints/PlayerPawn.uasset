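; Player pawn that runs a lane-dodging car game, moving the PlayerCarModel between RoadPlane lanes with A/D through a timeline lerp.
; GameControl creates the score UI and runs looping delayed spawns of cars and energy pickups on the plane, while MakeGameHarder changes spawn and speed settings in timed stages.
; Tick drains energy and adds score through delays; on death it saves a new high score, shows EndScreen and pauses.
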(event Custom|Game%20Control
  ;[1 1 1] Game controlling
  (Utilities|FlowControl|Sequence
    (:then_0
      (CallFunction|CreateUI))
    (:then_1
      ;;[1 1 1] Looping Spawn
      (Utilities|FlowControl|Delay (Math|Random|RandomFloatinRange (Variables|Default|GetCarMinimumSpawnTime) (Variables|Default|GetCarMaximumSpawnTime)) :!label _label)
      (Default|SpawnCar (Variables|Default|GetPlane) (Math|Random|RandomIntegerinRange 0 3) false (Variables|Default|GetMinimalSpeed) (Variables|Default|GetMaximalSpeed))
      (goto _label))
    (:then_2
      ;;[1 1 1] Energy SpawnTime
      (Utilities|FlowControl|Delay (Variables|Default|GetEnergySpawnTime) :!label _label_2)
      (Default|SpawnCar (Variables|Default|GetPlane) (Math|Random|RandomIntegerinRange 0 3) true 0.0 0.0)
      (goto _label_2))
    (:then_3
      (CallFunction|MakeGameHarder))))

(event Custom|Full%20Energy
  ;[1 1 1] Making full energy
  (Variables|Default|SetEnergy (Variables|Default|GetMaxEnergy)))

(event Custom|MakeGameHarder
  ;[1 1 1] Game Controlling
  (Utilities|FlowControl|Delay 1e+01)
  (Variables|Default|SetCarMinimumSpawnTime 2.0)
  (Variables|Default|SetCarMaximumSpawnTime 4.0)
  (Variables|Default|SetEnergyTimeSpawn 1e+01)
  (Variables|Default|SetMinimalSpeed -0.3)
  (Variables|Default|SetMaximalSpeed -0.5)
  (Utilities|FlowControl|Delay 2e+01)
  (Variables|Default|SetCarMinimumSpawnTime 1.0)
  (Variables|Default|SetCarMaximumSpawnTime 3.0)
  (Variables|Default|SetEnergyTimeSpawn 17.0)
  (Variables|Default|SetMinimalSpeed -1.0)
  (Variables|Default|SetMaximalSpeed -3.0))

(event EventBeginPlay
  ;[1 1 1] Initial conditions
  (Utilities|FlowControl|Sequence
    (:then_0
      (bind _ascar_game_instance (Utilities|Casting|CastToCarGameInstance (Game|GetGameInstance)))
      (Variables|Default|SetGameInstance _ascar_game_instance))
    (:then_1
      (bind _outactors (Actor|GetAllActorsOfClass "/Game/Blueprints/PlayerCarModel.PlayerCarModel_C"))
      (Variables|Default|SetCar (Utilities|Array|Get(acopy) _outactors))
      (Variables|Default|SetCarPositionNum 1)
      (bind _outactors_2 (Actor|GetAllActorsOfClass "/Game/Blueprints/RoadPlane.RoadPlane_C"))
      (Variables|Default|SetPlane (Utilities|Array|Get(acopy) _outactors_2))
      (bind _return (Default|PositionFunc (Variables|Default|GetPlane) (Variables|Default|GetCarPositionNum)))
      (Transformation|SetActorLocation (Variables|Default|GetCar) _return false false)
      (CallFunction|GameControl))))

(event EventTick
  (params (DeltaSeconds :type Float%20%28single-precision%29))
  (bind _gameinstance (Variables|Default|GetGameInstance))
  ;[1 1 1] Tick moments
  (if (!= (Variables|Default|GetCar) 0)
    (if (Variables|/Game/Blueprints/PlayerCarModel.PlayerCarModel_C|GetIsDead (Variables|Default|GetCar))
      (Utilities|FlowControl|DoOnce false
        (:Completed
          (Utilities|FlowControl|Sequence
            (:then_0
              (if (> (Variables|Default|GetPlayerScore) (Variables|/Game/Blueprints/CarGameInstance.CarGameInstance_C|GetScore _gameinstance))
                (Variables|/Game/Blueprints/CarGameInstance.CarGameInstance_C|SetScore _gameinstance (Variables|Default|GetPlayerScore))
                (Default|SaveScore _gameinstance)))
            (:then_1
              (bind _returnvalue (UserInterface|CreateWidget "/Game/UI/EndScreen.EndScreen_C"))
              (UserInterface|Viewport|AddtoViewport _returnvalue 0)
              (Variables|/Script/Engine.PlayerController|SetbShowMouseCursor (Game|GetPlayerController 0) true)
              (Utilities|FlowControl|Delay 0.2)
              (Game|SetGamePaused true)))))
      (else
        (Utilities|FlowControl|Sequence
          (:then_0
            (Utilities|FlowControl|Delay 0.2)
            (Variables|Default|SetEnergy (- (Variables|Default|GetEnergy) 0.5))
            (if (<= (Variables|Default|GetEnergy) 0.0)
              (Variables|/Game/Blueprints/PlayerCarModel.PlayerCarModel_C|SetIsDead (Variables|Default|GetCar) true)))
          (:then_1
            (Utilities|FlowControl|Delay 0.2)
            (Variables|Default|SetPlayerScore (+ (Variables|Default|GetPlayerScore) 1))))))))

(event Input|KeyboardEvents|A
  (params (Key :type Key%20Structure))
  ;[1 1 1] Input
  (:Pressed
    (if (not (Audio|Components|Audio|IsPlaying (Variables|Default|GetTransitionTimeline)))
      (if (!= (Variables|Default|GetCarPositionNum) 1)
        (Variables|Default|SetCarPositionNum (- (Variables|Default|GetCarPositionNum) 1))
        (bind _return (Default|PositionFunc (Variables|Default|GetPlane) (Variables|Default|GetCarPositionNum)))
        (bind _output_get (Variables|Default|SetCarOldLocation (Transformation|GetActorLocation (Variables|Default|GetCar))))
        (bind _alpha (Timeline|TransitionTimeline PlayFromStart)
          (:Update
            (Transformation|SetActorLocation (Variables|Default|GetCar) (Math|Vector|Lerp(Vector) _output_get _return _alpha) false false)))))))

(event Input|KeyboardEvents|D
  (params (Key :type Key%20Structure))
  ;[1 1 1] Input
  (:Pressed
    (if (not (Audio|Components|Audio|IsPlaying (Variables|Default|GetTransitionTimeline)))
      (if (!= (Variables|Default|GetCarPositionNum) (Variables|Default|GetMaxCarPosition))
        (Variables|Default|SetCarPositionNum (+ (Variables|Default|GetCarPositionNum) 1))
        (bind _return (Default|PositionFunc (Variables|Default|GetPlane) (Variables|Default|GetCarPositionNum)))
        (bind _output_get (Variables|Default|SetCarOldLocation (Transformation|GetActorLocation (Variables|Default|GetCar))))
        (bind _alpha (Timeline|TransitionTimeline PlayFromStart)
          (:Update
            (Transformation|SetActorLocation (Variables|Default|GetCar) (Math|Vector|Lerp(Vector) _output_get _return _alpha) false false)))))))

(fn ConstructionScript)

(fn CreateUI
  (bind _returnvalue (UserInterface|CreateWidget "/Game/UI/ScoreUI.ScoreUI_C"))
  (UserInterface|Viewport|AddtoViewport _returnvalue 0))