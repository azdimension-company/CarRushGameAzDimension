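; RoadPlane is a four-lane road that spawns enemy cars and energy pickups at per-lane spawn points.
; SpawnCar skips the requested lane if IsCarIsOnRoad finds an existing EnemyCarModel with that RoadIndex, scanning all such actors.
; Otherwise it spawns either Energy or an enemy car, which receives its lane index and a random speed within the given range.
; PositionFunc separately maps positions one to four to component world locations.
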(event Custom|Spawn%20Car
  (params (Position :type Integer) (IsItEnergy? :type Boolean) (MinimalSpeed :type Float%20%28single-precision%29) (MaximumSpeed :type Float%20%28single-precision%29))
  (bind _cannotbepassed (CallFunction|IsCarIsonRoad? Position))
  (if (not _cannotbepassed)
    (switch int Position
      (:0
        (Variables|Default|SetLocationOfEnemy (Transformation|GetWorldLocation (Variables|Default|GetEnemyPos1)))
        (Variables|Default|SetRoadIndex 0))
      (:1
        (Variables|Default|SetLocationOfEnemy (Transformation|GetWorldLocation (Variables|Default|GetEnemyPos2)))
        (Variables|Default|SetRoadIndex 1))
      (:2
        (Variables|Default|SetLocationOfEnemy (Transformation|GetWorldLocation (Variables|Default|GetEnemyPos3)))
        (Variables|Default|SetRoadIndex 2))
      (:3
        (Variables|Default|SetLocationOfEnemy (Transformation|GetWorldLocation (Variables|Default|GetEnemyPos4)))
        (Variables|Default|SetRoadIndex 3)))
    (if IsItEnergy?
      (Game|SpawnActorfromClass "/Game/Blueprints/Energy.Energy_C" (Math|Transform|MakeTransform (Variables|Default|GetLocationOfEnemy)) "Undefined" 0 0)
      (else
        (Game|SpawnActorfromClass "/Game/Blueprints/EnemyCarModel.EnemyCarModel_C" (Math|Transform|MakeTransform (Variables|Default|GetLocationOfEnemy)) "Undefined" 0 (Math|Random|RandomFloatinRange MinimalSpeed MaximumSpeed) (Variables|Default|GetRoadIndex) 0)))))

(fn ConstructionScript)

(fn PositionFunc
  (params (Position :type Integer))
  (switch int Position
    (:1
      (return (Transformation|GetWorldLocation (Variables|Default|Get1))))
    (:2
      (return (Transformation|GetWorldLocation (Variables|Default|Get2))))
    (:3
      (return (Transformation|GetWorldLocation (Variables|Default|Get3))))
    (:4
      (return (Transformation|GetWorldLocation (Variables|Default|Get4))))))

(fn IsCarIsonRoad?
  (params (Position :type Integer))
  (bind _outactors (Actor|GetAllActorsOfClass "/Game/Blueprints/EnemyCarModel.EnemyCarModel_C"))
  (for _array_element _outactors
    (if (== Position (Variables|/Game/Blueprints/EnemyCarModel.EnemyCarModel_C|GetRoadIndex _array_element))
      (LocalVariables|SetWasFound true)))
  (return (LocalVariables|GetWasFound)))