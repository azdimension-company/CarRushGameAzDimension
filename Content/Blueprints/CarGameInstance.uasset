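; CarGameInstance is the game instance that holds the car game's Score and persists it through a SaveGameClass object in the "Score" slot.
; On Init the branch runs inverted: an existing save is overwritten with a new object, while a missing one triggers a load whose cast then fails.
; SaveScore loads the slot, writes the current Score and saves it back, doing nothing if the cast fails.
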(event Custom|Save%20Score
  (bind _returnvalue (SaveGame|LoadGamefromSlot "Score"))
  (bind _assave_game_class (Utilities|Casting|CastToSaveGameClass _returnvalue))
  (Variables|/Game/Blueprints/SaveGameClass.SaveGameClass_C|SetScore _assave_game_class (Variables|Default|GetScore))
  (SaveGame|SaveGametoSlot _assave_game_class "Score"))

(event EventInit
  (bind _returnvalue (SaveGame|DoesSaveGameExist "Score"))
  (if _returnvalue
    (bind _returnvalue_2 (SaveGame|CreateSaveGameObject "/Game/Blueprints/SaveGameClass.SaveGameClass_C"))
    (bind _output_get (Variables|Default|SetSaveGameObject _returnvalue_2))
    (SaveGame|SaveGametoSlot _output_get "Score")
    (else
      (bind _returnvalue_3 (SaveGame|LoadGamefromSlot "Score"))
      (bind _assave_game_class (Utilities|Casting|CastToSaveGameClass _returnvalue_3))
      (Variables|Default|SetScore (Variables|/Game/Blueprints/SaveGameClass.SaveGameClass_C|GetScore _assave_game_class)))))